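; BP_Motor_Ctrl is a motor controller that sends motion commands to SimCorDX over local UDP using ObjectDeliverer, identifying itself as TankUE.
; It repeats the ID every three seconds and each tick sends a "~M" string built from a timeline driven by Move Right.
; Separately, held A/D keys ramp a clamped Speed, which indexes smoothstep timelines to produce SmoothSpeed, which is only printed, not sent.
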(event Custom|Connected
  (params (ClientSocket :type Object%20Deliverer%20Protocol%20Object%20Reference))
  (Development|PrintString "Connected to SimCorDX"))

(event Custom|Disconnected
  (params (ClientSocket :type Object%20Deliverer%20Protocol%20Object%20Reference))
  (Development|PrintString "Disconnected from SimCorDX"))

(event Custom|Received
  (params (ReceivedString :type String) (FromObject :type Object%20Deliverer%20Protocol%20Object%20Reference))
  (Development|PrintString (Utilities|String|Append "SimCorDX Says" ReceivedString)))

(event EventBeginPlay
  (bind _returnvalue (Utilities|String|Append "#id " "TankUE" "\\n"))
  ;[1 1 1] Enable Input on begin play
  (Input|EnableInput (Game|GetPlayerController 0))
  (bind _output_get (Variables|Default|SetObjDelMng (Class|ObjectDelivererManager|CreateObjectDelivererManager true)))
  (EventDispatchers|BindEventtoConnected _output_get (delegate Custom|Connected))
  (EventDispatchers|BindEventtoDisconnected (Variables|Default|GetObjDelMng) (delegate Custom|Disconnected))
  (bind _output_get_2 (Variables|Default|SetDeliveryBox (Class|DeliveryBoxFactory|CreateUtf8StringDeliveryBox)))
  (EventDispatchers|BindEventtoReceived _output_get_2 (delegate Custom|Received))
  (Class|ObjectDelivererManager|Start (Variables|Default|GetObjDelMng) (Class|ProtocolFactory|CreateProtocolUdpSocketSender "127.0.0.1" 1288) (Class|PacketRuleFactory|CreatePacketRuleNodivision) (Variables|Default|GetDeliveryBox))
  ;[1 1 1 0.1627] Send #ID message
  (Class|Utf8StringDeliveryBox|Send (Variables|Default|GetDeliveryBox) _returnvalue :!label _label)
  (Development|PrintString _returnvalue true true "(R=0.055069,G=1.000000,B=0.000000,A=1.000000)")
  (Utilities|FlowControl|Delay 3.0)
  (goto _label))

(event EventTick
  (params (DeltaSeconds :type Float%20%28single-precision%29))
  (bind _returnvalue (Utilities|Time|GetWorldDeltaSeconds))
  (bind _speed (Variables|Default|GetSpeed))
  (Class|Utf8StringDeliveryBox|Send (Variables|Default|GetDeliveryBox) (Utilities|String|Append "~M" "000" (Utilities|String|Append "0" "0" (Utilities|String|ToString(Float) (* (stale Input|AxisEvents|InputAxisMoveRight _newtrack_0) 1e+01)))))
  (Development|PrintString (Utilities|String|Append "~M" "000" (Utilities|String|Append "0" "0" (Utilities|String|ToString(Float) (* (stale Input|AxisEvents|InputAxisMoveRight _newtrack_0) 1e+01)))))
  ;[0.1875 1 0 0.139] Comment
  (if (> _speed 0.0)
    (bind _smoothstep (Timeline|SmoothStep SetNewTime)
      (:Update
        (Variables|Default|SetSmoothSpeed _smoothstep)))
    (else
      (bind _smoothstep_2 (Timeline|Timeline1 SetNewTime)
        (:Update
          (bind _output_get (Variables|Default|SetSmoothSpeed (* _smoothstep_2 -1.0)))))))
  (Development|PrintString (Utilities|String|ToString(Float) _output_get) true true "(R=0.000000,G=0.660000,B=1.000000,A=1.000000)" _returnvalue)
  (Development|PrintString (Utilities|String|ToString(Float) (Variables|Default|GetSpeed)) true true "(R=0.000000,G=0.660000,B=1.000000,A=1.000000)" _returnvalue))

(event Input|AxisEvents|InputAxisMoveRight
  (params (AxisValue :type Float%20%28single-precision%29))
  (if (> AxisValue 0.0)
    (bind _newtrack_0 (Timeline|Timeline Play))
    (else
      (Timeline|Timeline Reverse))))

(event Input|KeyboardEvents|A
  (params (Key :type Key%20Structure))
  ;[0 0.0145 1 0.122] Comment
  (:Pressed
    (Variables|Default|SetTurningRight true)
    (if (Variables|Default|GetTurningRight) :!label _label
      (Variables|Default|SetSpeed (+ (Variables|Default|GetSpeed) 0.1))
      (if (> (Variables|Default|GetSpeed) 1.0)
        (Variables|Default|SetSpeed 1.0))
      (Utilities|FlowControl|Delay 0.02)
      (goto _label)))
  (:Released
    (Variables|Default|SetTurningRight false)))

(event Input|KeyboardEvents|D
  (params (Key :type Key%20Structure))
  ;[0 0.0145 1 0.122] Comment
  (:Pressed
    (Variables|Default|SetTurningLeft true)
    (if (Variables|Default|GetTurningLeft) :!label _label
      (Variables|Default|SetSpeed (+ (Variables|Default|GetSpeed) -0.1))
      (if (< (Variables|Default|GetSpeed) -1.0)
        (Variables|Default|SetSpeed -1.0))
      (Utilities|FlowControl|Delay 0.02)
      (goto _label)))
  (:Released
    (Variables|Default|SetTurningLeft false)))

(fn ConstructionScript)